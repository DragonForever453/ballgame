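; BP_Boost is a boost pad actor that pushes components entering its Box trigger along the BoostDirection forward vector.
; When IsOneTime is set, overlap applies a single velocity-change impulse scaled by Speed.
; Otherwise, Tick applies that impulse scaled by delta time while IsBoosting is true, until end overlap clears the flag.
; Only the most recent overlap's component is pushed, and any end overlap stops the continuous boost.
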(event OnComponentBeginOverlap(Box)
  (params (OverlappedComponent :type Primitive%20Component%20Object%20Reference) (OtherActor :type Actor%20Object%20Reference) (OtherComp :type Primitive%20Component%20Object%20Reference) (OtherBodyIndex :type Integer) (bFromSweep :type Boolean) (SweepResult :type Hit%20Result%20Structure%20%28by%20ref%29))
  (Variables|Default|SetOther%20Comp OtherComp)
  (Variables|Default|SetIsBoosting true)
  (if (Variables|Default|GetIsOneTime)
    (Physics|AddImpulse (Variables|Default|GetOther%20Comp) (* (Math|Vector|GetForwardVector (Variables|Default|GetBoostDirection)) (Variables|Default|GetSpeed)) "None" true)))

(event OnComponentEndOverlap(Box)
  (params (OverlappedComponent :type Primitive%20Component%20Object%20Reference) (OtherActor :type Actor%20Object%20Reference) (OtherComp :type Primitive%20Component%20Object%20Reference) (OtherBodyIndex :type Integer))
  (Variables|Default|SetIsBoosting false))

(event EventBeginPlay)

(event Collision|EventActorBeginOverlap
  (params (OtherActor :type Actor%20Object%20Reference)))

(event EventTick
  (params (DeltaSeconds :type Float%20%28single-precision%29))
  (Variables|Default|SetDelta%20Seconds DeltaSeconds)
  (if (not (Variables|Default|GetIsOneTime))
    (if (Variables|Default|GetIsBoosting)
      (Physics|AddImpulse (Variables|Default|GetOther%20Comp) (* (* (Math|Vector|GetForwardVector (Variables|Default|GetBoostDirection)) (Variables|Default|GetSpeed)) (Variables|Default|GetDelta%20Seconds)) "None" true))))

(fn ConstructionScript)