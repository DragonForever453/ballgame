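; BP_Ball1 is a player-controlled ball driven by physics impulses.
; BeginPlay adds the IMC_Player Enhanced Input context, and IA_Camera feeds controller pitch and yaw.
; IA_Move turns normalized input into a Speed-scaled, velocity-change impulse on the Sphere, relative to camera yaw.
; WASD and Space still set direction flags, but the fixed-impulse logic reading them is disconnected, leaving Space without effect.
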(event Input|EnhancedActionEvents|EnhancedInputActionIA_Move
  (params (ActionValue :type Vector%202D%20Structure) (ElapsedSeconds :type Float%20%28double-precision%29) (TriggeredSeconds :type Float%20%28double-precision%29) (InputAction :type Input%20Action%20Object%20Reference :default "/Game/IA_Move.IA_Move"))
  (bind _returnvalue (Pawn|GetControlRotation :!class /Script/Engine.Pawn))
  (bind _returnvalue_2 (Math|Vector2D|Normalize2D ActionValue))
  (bind _returnvalue_3 (Math|Rotator|MakeRotator 0.0 0.0 (.yaw _returnvalue)))
  (Physics|AddImpulse (Variables|Default|GetSphere) (* (+ (* (.x _returnvalue_2) (Math|Vector|GetRightVector _returnvalue_3)) (* (.y _returnvalue_2) (Math|Vector|GetForwardVector _returnvalue_3))) (Variables|Default|Getspeed)) "None" true))

(event Input|EnhancedActionEvents|EnhancedInputActionIA_Camera
  (params (ActionValue :type Vector%202D%20Structure) (ElapsedSeconds :type Float%20%28double-precision%29) (TriggeredSeconds :type Float%20%28double-precision%29) (InputAction :type Input%20Action%20Object%20Reference :default "/Game/IA_Camera.IA_Camera"))
  (:Triggered
    (Pawn|Input|AddControllerPitchInput (.x ActionValue))
    (Pawn|Input|AddControllerYawInput (.y ActionValue))))

(event Collision|EventActorBeginOverlap
  (params (OtherActor :type Actor%20Object%20Reference)))

(event EventTick
  (params (DeltaSeconds :type Float%20%28single-precision%29)))

(event EventBeginPlay
  (Input|AddMappingContext (PlayerController|LocalPlayerSubsystems|GetEnhancedInputLocalPlayerSubsystem (Game|GetPlayerController 0)) "/Game/IMC_Player.IMC_Player" 0 "(bIgnoreAllPressedKeysUntilRelease=True,bForceImmediately=False,bNotifyUserSettings=False)"))

(event Input|KeyboardEvents|W
  (params (Key :type Key%20Structure :default "None"))
  (:Pressed
    (Variables|Default|Setforward true))
  (:Released
    (Variables|Default|Setforward false)))

(event Input|KeyboardEvents|S
  (params (Key :type Key%20Structure :default "None"))
  (:Pressed
    (Variables|Default|Setbackward true))
  (:Released
    (Variables|Default|Setbackward false)))

(event Input|KeyboardEvents|D
  (params (Key :type Key%20Structure :default "None"))
  (:Pressed
    (Variables|Default|Setright true))
  (:Released
    (Variables|Default|Setright false)))

(event Input|KeyboardEvents|A
  (params (Key :type Key%20Structure :default "None"))
  (:Pressed
    (Variables|Default|Setleft true))
  (:Released
    (Variables|Default|Setleft false)))

(event Input|KeyboardEvents|SpaceBar
  (params (Key :type Key%20Structure :default "None"))
  (:Pressed
    (Variables|Default|Setup true))
  (:Released
    (Variables|Default|Setup false)))

(fn ConstructionScript)